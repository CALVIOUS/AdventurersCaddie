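; Character Blueprint for Grungus, a hero in the adventure scene.
; Every tick it resets the actor's location to the capsule's X and Y with Z taken from CharacterZValue, pinning it to that height without sweeping.
; A Death event disables movement and turns on collision and physics simulation for all skeletal mesh bodies, ragdolling the character.
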(event Custom|Death
  (bind _skeletalmesh (Variables|Default|GetSkeletalMesh))
  (Pawn|Components|CharacterMovement|DisableMovement (Variables|Character|GetCharacterMovement))
  (Collision|SetCollisionEnabled _skeletalmesh "QueryAndPhysics")
  (Class|SkeletalMeshComponent|SetAllBodiesSimulatePhysics _skeletalmesh true))

(event EventBeginPlay)

(event Collision|EventActorBeginOverlap
  (params (OtherActor :type Actor%20Object%20Reference)))

(event EventTick
  (params (DeltaSeconds :type Float%20%28single-precision%29))
  (bind _capsulecomponent (Variables|Collision|GetCapsuleComponent))
  (bind _returnvalue (Transformation|GetWorldLocation _capsulecomponent))
  (bind (_x _y) (Math|Vector|BreakVector _returnvalue))
  (Variables|Default|SetDeltaSeconds DeltaSeconds)
  (Transformation|SetActorLocation (Math|Vector|MakeVector _x _y (Variables|Default|GetCharacterZValue)) false false))

(fn ConstructionScript)