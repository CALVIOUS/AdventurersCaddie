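; Health potion item model for the adventure scene that flies to Grungus and triggers the potion's effect.
; On BeginPlay it moves its root component to the location and rotation of the first Grungus_BP found.
; It then calls HealthPotionEffect on the card game player controller and destroys itself.
; An unconnected SpawnActor node, noted for an explosion effect, never runs.
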(event EventBeginPlay
  (|CallParentFunction)
  (bind _outactors (Actor|GetAllActorsOfClass "/Game/Blueprints/AdventureScene/Hero/Grungus_BP.Grungus_BP_C"))
  (Components|MoveComponentTo (Variables|Default|GetDefaultSceneRoot) (.location (Transformation|GetWorldTransform (Variables|/Script/Engine.Actor|GetRootComponent (Utilities|Array|Get(acopy) _outactors)))) (.rotation (Transformation|GetWorldTransform (Variables|/Script/Engine.Actor|GetRootComponent (Utilities|Array|Get(acopy) _outactors)))) false false 0.2 false)
  (bind _ascard_game_player_controller_bp (Utilities|Casting|CastToCardGamePlayerController_BP (Game|GetPlayerController 0)))
  (Default|HealthPotionEffect _ascard_game_player_controller_bp)
  (Actor|DestroyActor))

(event Collision|EventActorBeginOverlap
  (params (OtherActor :type Actor%20Object%20Reference))
  (|CallParentFunction OtherActor) ; This node is disabled and will not be called.\nDrag off pins to build functionality.
)

(event EventTick
  (params (DeltaSeconds :type Float%20%28single-precision%29))
  (|CallParentFunction DeltaSeconds) ; This node is disabled and will not be called.\nDrag off pins to build functionality.
)

(fn ConstructionScript
  (|CallParentFunction))