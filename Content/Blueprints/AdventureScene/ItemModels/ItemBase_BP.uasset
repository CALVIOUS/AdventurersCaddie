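; ItemBase_BP is the item model base for the adventure scene, handling items thrown to the hero, Grungus_BP.
; On BeginPlay, if ItemThrown is set, it moves its root to the transform of the first Grungus_BP's HeldItem.
; It then hands off by setting that HeldItem child actor component to its own class and destroying itself, so the held item is a fresh instance.
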(event EventBeginPlay
  ;[1 1 1] Throws Item to Hero and attaches it once it reaches the target
  (if (Variables|Default|GetItemThrown)
    (bind _outactors (Actor|GetAllActorsOfClass "/Game/Blueprints/AdventureScene/Hero/Grungus_BP.Grungus_BP_C"))
    (Components|MoveComponentTo (Variables|Default|GetDefaultSceneRoot) (.location (Transformation|GetWorldTransform (Variables|/Game/Blueprints/AdventureScene/Hero/Grungus_BP.Grungus_BP_C|GetHeldItem (Utilities|Array|Get(acopy) _outactors)))) (.rotation (Transformation|GetWorldTransform (Variables|/Game/Blueprints/AdventureScene/Hero/Grungus_BP.Grungus_BP_C|GetHeldItem (Utilities|Array|Get(acopy) _outactors)))) false false 0.2 false)
    (ChildActorComponent|SetChildActorClass (Variables|/Game/Blueprints/AdventureScene/Hero/Grungus_BP.Grungus_BP_C|GetHeldItem (Utilities|Array|Get(acopy) _outactors)) (Utilities|GetClass self))
    (Actor|DestroyActor)))

(event Collision|EventActorBeginOverlap
  (params (OtherActor :type Actor%20Object%20Reference)))

(event EventTick
  (params (DeltaSeconds :type Float%20%28single-precision%29)))

(fn ConstructionScript)