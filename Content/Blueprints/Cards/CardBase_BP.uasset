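; CardBase_BP is a card actor, named as a base for cards, that responds to mouse clicks on its CardModel component.
; A left click clears the zoom flag and passes the card to CardGamePlayerController_BP through CardClicked.
; A right click toggles zoom by moving the actor to ZoomPosition and back to its saved location, a feature noted as not yet working.
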(event OnClicked(CardModel)
  (params (TouchedComponent :type Primitive%20Component%20Object%20Reference) (ButtonPressed :type Key%20Structure :default "None"))
  (if (== ButtonPressed "LeftMouseButton")
    (Variables|Default|SetZoom false)
    (bind _ascard_game_player_controller_bp (Utilities|Casting|CastToCardGamePlayerController_BP (Game|GetPlayerController 0)))
    (Default|CardClicked _ascard_game_player_controller_bp self)
    (else
      ;[1 1 1] Zoom function yet to work
      (if (== ButtonPressed "RightMouseButton")
        (if (Variables|Default|GetZoom)
          (Variables|Default|SetZoom false)
          (Transformation|SetActorLocation (Variables|Default|GetLastPostion) false false)
          (else
            (Variables|Default|SetZoom true)
            (Variables|Default|SetLastPostion (Transformation|GetActorLocation))
            (Transformation|SetActorLocation (Variables|Default|GetZoomPosition) false false)))))))

(event EventBeginPlay)

(event Collision|EventActorBeginOverlap
  (params (OtherActor :type Actor%20Object%20Reference)))

(event EventTick
  (params (DeltaSeconds :type Float%20%28single-precision%29)))

(fn ConstructionScript)